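; Component named for slide, hook and wall-climb movement, though its graph only handles reference setup and attachment.
; The get_player event stores the Character, Hand and Gun references passed to it.
; The attach event checks the AttachmentAttached flag and, when true, calls Attach on the Gun, then AttachHand twice on the Hand.
; No slide, hook or climb logic appears in this graph.
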(event `get_player`
  (params (character :type "Character Object Reference") (hand :type "/Game/models/hand/hands_Blueprint Object Reference") (gun :type "/Game/models/gun/gun2/gun_Blueprint Object Reference"))
  (set `self.character` character)
  (set `self.hand` hand)
  (set `self.gun` gun))

(event `attach`
  (bind _hand (`self.hand`))
  ;[1 0 0.2409 1 75] Attachment
  (if (`self.attachment_attached`)
    (`/Game/models/gun/gun2/gun_Blueprint.attach` (`self.gun`))
    (`/Game/models/hand/hands_Blueprint.attach_hand` _hand)
    (`/Game/models/hand/hands_Blueprint.attach_hand` _hand)))